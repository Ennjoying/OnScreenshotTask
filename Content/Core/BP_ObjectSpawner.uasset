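; BP_ObjectSpawner is an actor that copies an object's class and scatters new instances of it across the visible scene.
; CopyObjectInCenter traces from the camera center, ignoring the player pawn, and saves the hit actor's class.
; SpawnObjectInViewport deprojects random screen positions into visibility traces and spawns the saved class at the hit locations with random yaw and slight fixed tilt.
; Both traces draw debug lines.
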(event Custom|SpawnObjectInViewport
  (params (Controller%20Reference :type BP%20PC%20Object%20Reference) (AmountToSpawn :type Integer))
  (bind _returnvalue (Viewport|GetViewportSize))
  (bind _returnvalue_2 (Math|Random|RandomFloat))
  (bind _returnvalue_3 (Math|Random|RandomFloat))
  (bind _returnvalue_4 (* _returnvalue_2 (.y _returnvalue)))
  (bind _returnvalue_5 (* _returnvalue_3 (.x _returnvalue)))
  (bind (_worldlocation _worlddirection) (Class|PlayerController|DeprojectScreenPositiontoWorld Controller%20Reference _returnvalue_5 _returnvalue_4))
  ;[1 1 1] Spawn Objects
  (for _index (range 0 (- AmountToSpawn 1))
    (bind _outhit (Collision|LineTraceByChannel _worldlocation (+ _worldlocation (* _worlddirection 1e+04)) "TraceTypeQuery1" false 0 "ForDuration" true "(R=1.000000,G=0.000000,B=0.000000,A=1.000000)" "(R=0.000000,G=1.000000,B=0.000000,A=1.000000)" 1.0))
    (Game|SpawnActorfromClass (Variables|Default|GetSavedObject) (Math|Transform|MakeTransform (.Location (Collision|BreakHitResult _outhit)) (Math|Rotator|MakeRotator 15.0 5.0 (* (Math|Random|RandomFloat) 3.6e+02)) "1.000000,1.000000,1.000000") "Undefined" "MultiplyWithRoot" 0 0)))

(event Custom|CopyObjectInCenter
  (bind _returnvalue (Game|GetPlayerCameraManager 0))
  (bind _returnvalue_2 (Camera|GetCameraLocation _returnvalue))
  ;[1 1 1] CopyObject
  (bind (_outhit _returnvalue_3) (Collision|LineTraceByChannel _returnvalue_2 (+ _returnvalue_2 (* (Math|Vector|GetForwardVector (Camera|GetCameraRotation _returnvalue)) 1e+03)) "TraceTypeQuery1" false (Variables|Default|GetActors%20to%20Ignore) "ForDuration" true "(R=1.000000,G=0.000000,B=0.000000,A=1.000000)" "(R=0.000000,G=1.000000,B=0.000000,A=1.000000)" 1.0))
  (if _returnvalue_3
    (Variables|Default|SetSavedObject (Utilities|GetClass (.HitActor (Collision|BreakHitResult _outhit))))
    (else
      (Development|PrintString "NoSpawnableObjectFound"))))

(event EventBeginPlay
  ;[1 1 1] Setup, so the Trace doesnt hit the Player Pawn
  (Utilities|Array|AddUnique (Variables|Default|GetActors%20to%20Ignore) (Game|Player|GetPlayerPawn 0)))

(fn ConstructionScript)