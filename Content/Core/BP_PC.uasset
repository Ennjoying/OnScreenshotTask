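; BP_PC is the player controller that handles hotkeys for object copy/paste and screenshots.
; On begin play it caches the BP_ObjectSpawner and adds the IMC_Standard Enhanced Input context.
; Copy and paste inputs delegate to the spawner, passing a clamped copy count that increment and decrement inputs adjust.
; The screenshot input ensures an On/Screenshots user directory exists, then takes a 1080p capture named by timestamp alone.
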(event Input|EnhancedActionEvents|EnhancedInputActionIA_TakeScreenshot
  (params (ActionValue :type Boolean) (ElapsedSeconds :type Float%20%28double-precision%29) (TriggeredSeconds :type Float%20%28double-precision%29) (InputAction :type Input%20Action%20Object%20Reference :default "/Game/Core/Inputs/IA_TakeScreenshot.IA_TakeScreenshot"))
  (bind _returnvalue (Math|DateTime|Now))
  (bind _returnvalue_2 (Class|BlueprintFileUtilsBPLibrary|GetUserDirectory))
  (bind _returnvalue_3 (Utilities|String|Append _returnvalue_2 "On/Screenshots"))
  ;[1 1 1] Screenshot logic
  (:Completed
    (if (Utilities|Paths|DirectoryExists _returnvalue_3)
      (Class|AutomationBlueprintFunctionLibrary|TakeHighResScreenshot 1920 1080 (Utilities|String|Append (Utilities|String|ToString(Integer) (.year _returnvalue)) "_" (Utilities|String|ToString(Integer) (.month _returnvalue)) "_" (Utilities|String|ToString(Integer) (.day _returnvalue)) "-" (Utilities|String|ToString(Integer) (.hour _returnvalue)) "_" (Utilities|String|ToString(Integer) (.minute _returnvalue)) "_" (Utilities|String|ToString(Integer) (.second _returnvalue))) 0 false false "Low" "" 0.0 :!label _label)
      (else
        (bind _returnvalue_4 (Class|BlueprintFileUtilsBPLibrary|MakeDirectory _returnvalue_3 true))
        (if _returnvalue_4
          (goto _label)
          (else
            (Development|PrintString (Utilities|String|Append "couldnt create Directory: " _returnvalue_3))))))))

(event Input|EnhancedActionEvents|EnhancedInputActionIA_CopyObject
  (params (ActionValue :type Boolean) (ElapsedSeconds :type Float%20%28double-precision%29) (TriggeredSeconds :type Float%20%28double-precision%29) (InputAction :type Input%20Action%20Object%20Reference :default "/Game/Core/Inputs/IA_CopyObject.IA_CopyObject"))
  ;[1 1 1] Copy & Paste Object triggers
  (:Completed
    (Default|CopyObjectinCenter (Variables|Default|GetObjectSpawnerRef))))

(event Input|EnhancedActionEvents|EnhancedInputActionIA_IncrementCopies
  (params (ActionValue :type Boolean) (ElapsedSeconds :type Float%20%28double-precision%29) (TriggeredSeconds :type Float%20%28double-precision%29) (InputAction :type Input%20Action%20Object%20Reference :default "/Game/Core/Inputs/IA_IncrementCopies.IA_IncrementCopies"))
  ;[1 1 1] Increment & Decrement copy amount
  (:Completed
    (Variables|Default|SetAmount%20to%20Spawn (Math|Integer|Clamp(Integer) (+ (Variables|Default|GetAmount%20to%20Spawn) 1) 0 15))))

(event Input|EnhancedActionEvents|EnhancedInputActionIA_PasteObject
  (params (ActionValue :type Boolean) (ElapsedSeconds :type Float%20%28double-precision%29) (TriggeredSeconds :type Float%20%28double-precision%29) (InputAction :type Input%20Action%20Object%20Reference :default "/Game/Core/Inputs/IA_PasteObject.IA_PasteObject"))
  ;[1 1 1] Copy & Paste Object triggers
  (:Completed
    (Default|SpawnObjectinViewport (Variables|Default|GetObjectSpawnerRef) self (Variables|Default|GetAmount%20to%20Spawn))))

(event Input|EnhancedActionEvents|EnhancedInputActionIA_DecrementCopies
  (params (ActionValue :type Boolean) (ElapsedSeconds :type Float%20%28double-precision%29) (TriggeredSeconds :type Float%20%28double-precision%29) (InputAction :type Input%20Action%20Object%20Reference :default "/Game/Core/Inputs/IA_DecrementCopies.IA_DecrementCopies"))
  ;[1 1 1] Increment & Decrement copy amount
  (:Completed
    (Variables|Default|SetAmount%20to%20Spawn (Math|Integer|Clamp(Integer) (- (Variables|Default|GetAmount%20to%20Spawn) 1) 0 15))))

(event EventBeginPlay
  ;[1 1 1] Setup
  (bind _returnvalue (Actor|GetActorOfClass "/Game/Core/BP_ObjectSpawner.BP_ObjectSpawner_C"))
  (Variables|Default|SetObjectSpawnerRef _returnvalue)
  (Input|AddMappingContext (PlayerController|LocalPlayerSubsystems|GetEnhancedInputLocalPlayerSubsystem self) "/Game/Core/Inputs/IMC_Standard.IMC_Standard" 0 "(bIgnoreAllPressedKeysUntilRelease=True,bForceImmediately=False,bNotifyUserSettings=False)"))

(fn ConstructionScript)